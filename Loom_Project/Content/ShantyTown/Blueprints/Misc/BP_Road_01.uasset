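; Road actor for ShantyTown that builds a road from spline mesh segments along its SplineTrack.
; The Construction Script splits the spline into sections of fixed length derived from actor X scale, dropping any leftover shorter than a full section.
; Each collision-enabled segment takes local-space endpoints and tangents from the spline, with tangent magnitude clamped to the section length to follow curves cleanly.
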(fn ConstructionScript
  (bind _splinetrack (Variables|Default|GetSplineTrack))
  (bind _splinetrack_2 (Variables|Default|GetSplineTrack))
  (Variables|Default|SetSection%20Length (* (.x (Transformation|GetActorScale3D)) 1e+03))
  (for _index (range 0 (- (Math|Float|Truncate (/ (Spline|GetSplineLength (Variables|Default|GetSplineTrack)) (Variables|Default|GetSection%20Length))) 1))
    (bind _returnvalue (AddComponent|AddSplineMeshComponent false))
    (SplineMesh|SetForwardAxis _returnvalue "X" true)
    (Collision|SetCollisionEnabled _returnvalue "QueryAndPhysics")
    (SplineMesh|SetStartandEnd _returnvalue (Spline|GetLocationatDistanceAlongSpline _splinetrack (* _index (Variables|Default|GetSection%20Length)) "Local") (Math|Vector|ClampVectorSize (Spline|GetTangentatDistanceAlongSpline _splinetrack (* _index (Variables|Default|GetSection%20Length)) "Local") 0.0 (Variables|Default|GetSection%20Length)) (Spline|GetLocationatDistanceAlongSpline _splinetrack_2 (* (+ _index 1) (Variables|Default|GetSection%20Length)) "Local") (Math|Vector|ClampVectorSize (Spline|GetTangentatDistanceAlongSpline _splinetrack_2 (* (+ _index 1) (Variables|Default|GetSection%20Length)) "Local") 0.0 (Variables|Default|GetSection%20Length)) true :!class /Script/Engine.SplineMeshComponent)))